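; BP_Protagonist is the protagonist character Blueprint, which creates its own HUD when play begins.
; BeginPlay checks whether its controller is player controller 0 or its local role is AutonomousProxy, covering both server-side and owning-client cases.
; When either holds, it creates a BP_Hud widget, passes itself in through SetProtagonist and adds it to the viewport.
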(event `self.ReceiveBeginPlay`
  (if (or (== (`GameplayStatics.GetPlayerController` 0) (`self.GetController`)) (`|EnumEquality` (`self.GetLocalRole`) "ROLE_AutonomousProxy"))
    (bind _returnvalue (`|CreateWidget` "/Game/MyContent/UI/BP_Hud.BP_Hud_C"))
    (`/Game/MyContent/UI/BP_Hud.SetProtagonist` _returnvalue self)
    (`UserWidget.AddToViewport` _returnvalue 0)))

(fn `UserConstructionScript`)